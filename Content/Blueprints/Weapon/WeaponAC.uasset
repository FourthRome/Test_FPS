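; Weapon actor component that tracks ammo counts per weapon type.
; Current and maximum ammo live in maps keyed by weapon type; adding and using ammo both route through a setter that clamps the result between zero and that type's maximum.
; A check function reports whether a type holds at least a requested amount, and the event graph is unused.
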(event EventBeginPlay)

(event EventTick
  (params (DeltaSeconds :type Float%20%28single-precision%29)))

(fn AddAmmo
  (params (WeaponType :type WeaponType%20Enum :default "NewEnumerator4") (Value :type Integer))
  (CallFunction|SetAmmo WeaponType (+ (.Value (Utilities|Map|Find (Variables|Default|GetCurrentAmmo) WeaponType)) Value)))

(fn UseAmmo
  (params (WeaponType :type WeaponType%20Enum :default "NewEnumerator4") (Value :type Integer))
  (CallFunction|SetAmmo WeaponType (- (.Value (Utilities|Map|Find (Variables|Default|GetCurrentAmmo) WeaponType)) Value)))

(fn SetAmmo
  (params (WeaponType :type WeaponType%20Enum :default "NewEnumerator4") (Value :type Integer))
  (Utilities|Map|Add (Variables|Default|GetCurrentAmmo) WeaponType (Math|Integer|Clamp(Integer) Value 0 (.Value (Utilities|Map|Find (Variables|Default|GetMaxAmmo) WeaponType)))))

(fn CheckAmmo
  (params (WeaponType :type WeaponType%20Enum :default "NewEnumerator4") (Value :type Integer))
  (return (>= (.Value (Utilities|Map|Find (Variables|Default|GetCurrentAmmo) WeaponType)) Value)))