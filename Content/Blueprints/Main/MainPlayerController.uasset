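; MainPlayerController is the player controller that turns player input into movement, camera and jump actions for the main character.
; On BeginPlay it casts the controlled pawn to MainPlayerCharacter and caches it, printing a message if the cast fails.
; Movement axes, Jump and SwitchCameraView forward to that cached character, while LookUp and TurnAround apply pitch and yaw input on the controller itself.
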(event EventBeginPlay
  (bind _asmain_player_character (Utilities|Casting|CastToMainPlayerCharacter (Pawn|GetControlledPawn))
    (:then
      (Variables|Default|SetMainPlayerCharacter _asmain_player_character))
    (:CastFailed
      (Development|PrintString "Cast failed"))))

(event EventTick
  (params (DeltaSeconds :type Float%20%28single-precision%29)))

(event Input|ActionEvents|InputActionAction
  (params (Key :type Key%20Structure :default "None")))

(event Input|ActionEvents|InputActionFire
  (params (Key :type Key%20Structure :default "None")))

(event Input|ActionEvents|InputActionJump
  (params (Key :type Key%20Structure :default "None"))
  (:Pressed
    (Character|Jump (Variables|Default|GetMainPlayerCharacter))))

(event Input|ActionEvents|InputActionSwitchCameraView
  (params (Key :type Key%20Structure :default "None"))
  (:Pressed
    (Default|SwitchCameraView (Variables|Default|GetMainPlayerCharacter))))

(event Input|AxisEvents|InputAxisMoveForward
  (params (AxisValue :type Float%20%28single-precision%29))
  (Default|MoveForward (Variables|Default|GetMainPlayerCharacter) AxisValue))

(event Input|AxisEvents|InputAxisMoveRight
  (params (AxisValue :type Float%20%28single-precision%29))
  (Default|MoveRight (Variables|Default|GetMainPlayerCharacter) AxisValue))

(event Input|AxisEvents|InputAxisLookUp
  (params (AxisValue :type Float%20%28single-precision%29))
  (Class|PlayerController|AddPitchInput AxisValue))

(event Input|AxisEvents|InputAxisTurnAround
  (params (AxisValue :type Float%20%28single-precision%29))
  (Class|PlayerController|AddYawInput AxisValue))

(fn ConstructionScript)