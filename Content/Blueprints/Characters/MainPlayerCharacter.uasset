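; Main player character Blueprint that provides directional movement and switching between first- and third-person camera views.
; On BeginPlay it fills health to maximum through BioStatAC and starts in first-person view.
; MoveForward and MoveRight feed actor-relative vectors into a shared MoveInDirection helper that adds input to CharacterMovement.
; SwitchCameraView flips a boolean, activating one camera, deactivating the other and swapping visibility between two meshes to match the view.
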(event EventBeginPlay
  (CallFunction|CharacterInit))

(event Collision|EventActorBeginOverlap
  (params (OtherActor :type Actor%20Object%20Reference)))

(event EventTick
  (params (DeltaSeconds :type Float%20%28single-precision%29)))

(fn ConstructionScript)

(fn MoveForward
  (params (Value :type Float%20%28single-precision%29))
  (CallFunction|MoveinDirection (Transformation|GetActorForwardVector) Value))

(fn MoveRight
  (params (Value :type Float%20%28single-precision%29))
  (CallFunction|MoveinDirection (Transformation|GetActorRightVector) Value))

(fn MoveinDirection
  (params (Direction :type Vector) (Value :type Float%20%28single-precision%29))
  (Class|PawnMovementComponent|AddInputVector (Variables|Character|GetCharacterMovement) (* Direction Value) false))

(fn SwitchCameraView
  (if (Variables|Default|GetThirdPersonView)
    (CallFunction|ActivateFirstPersonCamera)
    (else
      (CallFunction|ActivateThirdPersonCamera)))
  (CallFunction|ToggleMeshesVisibility (Variables|Default|GetThirdPersonView))
  (Variables|Default|SetThirdPersonView (not (Variables|Default|GetThirdPersonView))))

(fn ToggleMeshesVisibility
  (params (SetFirstPersonMesh :type Boolean))
  (Rendering|SetVisibility (Variables|Character|GetMesh) SetFirstPersonMesh false)
  (Rendering|SetVisibility (Variables|Default|GetSkeletalMesh) (not SetFirstPersonMesh) false))

(fn ActivateFirstPersonCamera
  (Components|Activation|Activate (Variables|Default|GetFirstPersonCamera) false)
  (Components|Activation|Deactivate (Variables|Default|GetThirdPersonCamera)))

(fn ActivateThirdPersonCamera
  (Components|Activation|Activate (Variables|Default|GetThirdPersonCamera) false)
  (Components|Activation|Deactivate (Variables|Default|GetFirstPersonCamera)))

(fn CharacterInit
  (bind _biostatac (Variables|Default|GetBioStatAC))
  (Default|SetHealth _biostatac (Variables|/Game/Blueprints/Characters/BioStatAC.BioStatAC_C|GetMaxHealth _biostatac))
  (CallFunction|ActivateFirstPersonCamera)
  (Variables|Default|SetThirdPersonView false)
  (CallFunction|ToggleMeshesVisibility true))