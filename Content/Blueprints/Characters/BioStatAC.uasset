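; BioStatAC is a character stat component, going by its name and folder, that tracks health.
; SetHealth writes CurrentHealth clamped between zero and MaxHealth.
; Damage and Heal subtract or add a value and route the result through SetHealth, so both respect the same bounds.
; The event graph holds only disabled placeholder events, and the file contains no death or notification logic.
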(event EventBeginPlay)

(event EventTick
  (params (DeltaSeconds :type Float%20%28single-precision%29)))

(fn SetHealth
  (params (Value :type Float%20%28single-precision%29))
  (Variables|Default|SetCurrentHealth (Math|Float|Clamp(Float) Value 0.0 (Variables|Default|GetMaxHealth))))

(fn Damage
  (params (Value :type Float%20%28single-precision%29))
  (CallFunction|SetHealth (- (Variables|Default|GetCurrentHealth) Value)))

(fn Heal
  (params (Value :type Float%20%28single-precision%29))
  (CallFunction|SetHealth (+ Value (Variables|Default|GetCurrentHealth))))